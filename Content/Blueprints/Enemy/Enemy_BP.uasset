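; Stationary enemy that turns toward the player and fires projectiles when within range, and dies when hit by the player's sphere projectile.
; Tick uses a short Delay to throttle the distance check and aiming, then a longer Delay to pace Enemy_Projectile spawns aimed at the player pawn.
; Overlap on its Sphere component with a Sphere_Projectile destroys both the projectile and the enemy.
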(event OnComponentBeginOverlap(Sphere)
  (params (OverlappedComponent :type Primitive%20Component%20Object%20Reference) (OtherActor :type Actor%20Object%20Reference) (OtherComp :type Primitive%20Component%20Object%20Reference) (OtherBodyIndex :type Integer) (bFromSweep :type Boolean) (SweepResult :type Hit%20Result%20Structure%20%28by%20ref%29))
  (bind _assphere_projectile (Utilities|Casting|CastToSphere_Projectile OtherActor))
  (Actor|DestroyActor _assphere_projectile)
  (Actor|DestroyActor))

(event EventTick
  (params (DeltaSeconds :type Float%20%28single-precision%29))
  (bind _returnvalue (Game|GetPlayerCharacter 0))
  (bind _returnvalue_2 (Transformation|GetActorLocation))
  (Utilities|FlowControl|Delay 0.2)
  (Variables|Default|SetcanShoot (<= (Transformation|GetDistanceTo _returnvalue self) 1.5e+03))
  (if (Variables|Default|GetcanShoot)
    (Transformation|SetActorRotation (Math|Rotator|FindLookatRotation (Transformation|GetWorldLocation (Variables|Default|GetSphere1)) (Transformation|GetWorldLocation (Variables|/Script/Engine.Character|GetMesh _returnvalue))))
    (Utilities|FlowControl|Delay 2.0)
    (Game|SpawnActorfromClass "/Game/Blueprints/Projectile/Enemy_Projectile.Enemy_Projectile_C" (Math|Transform|MakeTransform _returnvalue_2 (Math|Rotator|FindLookatRotation _returnvalue_2 (Transformation|GetActorLocation (Game|Player|GetPlayerPawn 0))) "1,1,1") "Undefined" 0 0)))

(fn ConstructionScript)