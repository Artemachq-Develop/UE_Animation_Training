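; Player projectile that homes in on the closest actor tagged "Homing", leaving a trail as it flies.
; BeginPlay starts the trail and loops LockOn every half second, which feeds FindHomingTarget's result into the movement component's homing target.
; The search keeps its best distance in ClosestDistance, with no reset shown.
; Repeated Hit events end it with an explosion; otherwise LockOn's delay destroys it as a timeout.
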(event Custom|Lock%20On
  (bind _projectilemovement (Variables|Default|GetProjectileMovement))
  (bind _homing_target (CallFunction|FindHomingTarget))
  (Variables|/Script/Engine.ProjectileMovementComponent|SetHomingTargetComponent _projectilemovement _homing_target)
  (Variables|/Script/Engine.ProjectileMovementComponent|SetbIsHomingProjectile _projectilemovement true)
  (Utilities|FlowControl|Delay 1e+01)
  (Actor|DestroyActor))

(event Collision|EventHit
  (params (MyComp :type Primitive%20Component%20Object%20Reference) (Other :type Actor%20Object%20Reference) (OtherComp :type Primitive%20Component%20Object%20Reference) (bSelfMoved :type Boolean) (HitLocation :type Vector :default "0, 0, 0") (HitNormal :type Vector :default "0, 0, 0") (NormalImpulse :type Vector :default "0, 0, 0") (Hit :type Hit%20Result%20Structure%20%28by%20ref%29))
  (bind _result (Math|Integer|IncrementInt (Variables|Default|GetCounter))
    (:%20%20
      (if (>= _result 6)
        (Actor|DestroyActor)
        (Game|SpawnActorfromClass "/Game/StarterContent/Blueprints/Blueprint_Effect_Explosion.Blueprint_Effect_Explosion_C" (Math|Conversions|ToTransform(Vector) HitLocation) "Undefined" 0 0)
        (Effects|Particles|Trails|EndTrails (Variables|Default|GetTrail))))))

(event EventBeginPlay
  (Effects|Particles|Trails|BeginTrails (Variables|Default|GetTrail) "None" "None" "ETrailWidthMode_FromCentre" 0.0)
  (CallFunction|Lockon :!label _label)
  (Utilities|FlowControl|Delay 0.5)
  (goto _label))

(fn ConstructionScript)

(fn FindHomingTarget
  (bind _outactors (Actor|GetAllActorsOfClasswithTag "/Script/Engine.Actor" "Homing"))
  (for _array_element _outactors
    (if (< (Math|Vector|VectorLength (- (Transformation|GetActorLocation _array_element) (Transformation|GetActorLocation))) (Variables|Default|GetClosestDistance))
      (Variables|Default|SetClosestDistance (Math|Vector|VectorLength (- (Transformation|GetActorLocation _array_element) (Transformation|GetActorLocation))))
      (Variables|Default|SetHomingTarget _array_element)))
  (return (Actor|GetComponentbyClass (Variables|Default|GetHomingTarget) "/Script/Engine.SceneComponent")))