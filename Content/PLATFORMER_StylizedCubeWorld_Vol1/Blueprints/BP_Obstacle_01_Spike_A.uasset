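; Spike trap obstacle for the platformer that damages the player and raises its spikes when stepped into.
; On Box overlap by Player_Blueprint, a short delay precedes a fixed Health deduction on the player reference cached at BeginPlay.
; A timeline then lerps the Spike's relative height between SpikeDown and SpikeUp, reversing after a delay on overlap end.
; The construction script applies configurable meshes and a shared material to Spike and Base.
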(event OnComponentBeginOverlap(Box)
  (params (OverlappedComponent :type Primitive%20Component%20Object%20Reference) (OtherActor :type Actor%20Object%20Reference) (OtherComp :type Primitive%20Component%20Object%20Reference) (OtherBodyIndex :type Integer) (bFromSweep :type Boolean) (SweepResult :type Hit%20Result%20Structure%20%28by%20ref%29))
  (bind _character (Variables|Default|GetCharacter))
  (Utilities|Casting|CastToPlayer_Blueprint OtherActor)
  (Utilities|FlowControl|Delay 0.2)
  (Variables|/Game/Character/Player_Blueprint.Player_Blueprint_C|SetHealth _character (- (Variables|/Game/Character/Player_Blueprint.Player_Blueprint_C|GetHealth _character) 1e+01))
  (bind _newtrack_0 (Timeline|Spike_ Play)
    (:Update
      (Transformation|SetRelativeLocation (Variables|Default|GetSpike) (Math|Vector|Lerp(Vector) (Math|Vector|MakeVector 0.0 0.0 (Variables|Default|GetSpike%20Down)) (Math|Vector|MakeVector 0.0 0.0 (Variables|Default|GetSpike%20Up)) _newtrack_0) false false))))

(event OnComponentEndOverlap(Box)
  (params (OverlappedComponent :type Primitive%20Component%20Object%20Reference) (OtherActor :type Actor%20Object%20Reference) (OtherComp :type Primitive%20Component%20Object%20Reference) (OtherBodyIndex :type Integer))
  (Utilities|Casting|CastToPlayer_Blueprint OtherActor)
  (Utilities|FlowControl|Delay 1.0)
  (bind _newtrack_0 (Timeline|Spike_ Reverse)
    (:Update
      (Transformation|SetRelativeLocation (Variables|Default|GetSpike) (Math|Vector|Lerp(Vector) (Math|Vector|MakeVector 0.0 0.0 (Variables|Default|GetSpike%20Down)) (Math|Vector|MakeVector 0.0 0.0 (Variables|Default|GetSpike%20Up)) _newtrack_0) false false))))

(event EventBeginPlay
  (bind _asplayer_blueprint (Utilities|Casting|CastToPlayer_Blueprint (Game|GetPlayerCharacter 0)))
  (Variables|Default|SetCharacter _asplayer_blueprint))

(event Collision|EventActorBeginOverlap
  (params (OtherActor :type Actor%20Object%20Reference)))

(event EventTick
  (params (DeltaSeconds :type Float%20%28single-precision%29)))

(fn ConstructionScript
  (Rendering|Material|SetMaterial (Variables|Default|GetSpike) 0 (Variables|Default|GetMaterial))
  (Components|StaticMesh|SetStaticMesh (Variables|Default|GetSpike) (Variables|Default|GetStatic%20Mesh%20Spike))
  (Components|StaticMesh|SetStaticMesh (Variables|Default|GetBase) (Variables|Default|GetStatic%20Mesh%20Base)))